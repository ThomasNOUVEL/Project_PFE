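; BP_Pnj is an NPC that follows a timed daily routine of up to three moves.
; On BeginPlay it passes its three destinations to its AIC_PNJ controller, and SetDestination events record the actor's current location as each one.
; NewHour compares the time with three hour/minute slots, advancing MomentDeLaJournee and ordering the controller to the matching destination.
; Discution prints the dialogue line indexed by that day-moment counter.
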(event Custom|Set%20Destination%203
  (Variables|Default|SetDestination%203 (Transformation|GetActorLocation)))

(event Custom|Set%20Destination%201
  (Variables|Default|SetDestination%201 (Transformation|GetActorLocation)))

(event Custom|Set%20Destination%202
  (Variables|Default|SetDestination%202 (Transformation|GetActorLocation)))

(event EventBeginPlay
  (bind _asaic_pnj (Utilities|Casting|CastToAIC_PNJ (AI|GetAIController self)))
  (bind _output_get (Variables|Default|SetAs%20AIC%20PNJ _asaic_pnj))
  (Default|GuiveInformations _output_get (Variables|Default|GetDestination%201) (Variables|Default|GetDestination%202) (Variables|Default|GetDestination%203)))

(event EventNewHour
  (params (Hour :type Integer) (Minute :type Integer))
  (for _index (range 0 2)
    (if (== Hour (Utilities|Select :Index _index :Option%200 (Variables|Default|GetHour%20move%201) :Option%201 (Variables|Default|GetHour%20move%202) :Option%202 (Variables|Default|GetHour%20move%203)))
      (if (== Minute (Utilities|Select :Index _index :Option%200 (Variables|Default|Getminute%20move%201) :Option%201 (Variables|Default|Getminute%20move%202) :Option%202 (Variables|Default|Getminute%20move%203)))
        (Math|Integer|IncrementInt (Variables|Default|GetMoment%20de%20la%20journee)
          (:%20%20
            (Default|MovetoDestination (Variables|Default|GetAs%20AIC%20PNJ) _index)))))))

(event EventDiscution
  (Development|PrintText (Utilities|Array|Get(acopy) (Variables|Default|GetLigne%20de%20dialogue) (Variables|Default|GetMoment%20de%20la%20journee))))

(fn ConstructionScript)