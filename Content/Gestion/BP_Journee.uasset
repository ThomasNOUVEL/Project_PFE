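; Day-cycle manager that runs the game clock from hour 6 to 20 and tints the level's directional light by hour.
; A looping timer, pausable and resumable, advances minutes in six steps per hour and updates the WInfoJournee widget.
; Each tick before closing time broadcasts the time to all BPI_Hour actors.
; At 20h it reverses the eyelid (Paupieres) animation, then opens Lvl_ThirdPerson after a delay.
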(event Custom|Day%20Tic
  (bind _w_info_journee (Variables|Default|GetW%20info%20journee))
  (bind _w_info_journee_2 (Variables|Default|GetW%20info%20journee))
  (bind _result (Math|Integer|IncrementInt (Variables|Default|GetMinute%20of%20the%20hour))
    (:%20%20
      (if (> _result 5)
        (Variables|Default|SetMinute%20of%20the%20hour 0)
        (bind _result_2 (Math|Integer|IncrementInt (Variables|Default|GetHour%20of%20the%20day))
          (:%20%20
            (Rendering|Components|Light|SetLightColor (Variables|/Script/Engine.Light|GetLightComponent (Variables|Default|GetDirection%20light)) (Utilities|Select :Index _result_2 :Option%200 "" :Option%201 "" :Option%202 "" :Option%203 "" :Option%204 "" :Option%205 "" :Option%206 "" :Option%207 "(R=0.514918,G=0.473532,B=0.313989,A=1.000000)" :Option%208 "(R=0.656250,G=0.602840,B=0.399903,A=1.000000)" :Option%209 "(R=0.734375,G=0.682576,B=0.485758,A=1.000000)" :Option%2010 "(R=0.864583,G=0.816735,B=0.634929,A=1.000000)" :Option%2011 "(R=1.000000,G=0.946827,B=0.744792,A=1.000000)" :Option%2012 "(R=1.000000,G=0.954423,B=0.781250,A=1.000000)" :Option%2013 "(R=1.000000,G=0.930550,B=0.666667,A=1.000000)" :Option%2014 "(R=1.000000,G=0.942486,B=0.723958,A=1.000000)" :Option%2015 "(R=0.906250,G=0.850195,B=0.637207,A=1.000000)" :Option%2016 "(R=0.703125,G=0.645900,B=0.428467,A=1.000000)" :Option%2017 "(R=0.640625,G=0.577363,B=0.336995,A=1.000000)" :Option%2018 "(R=0.375000,G=0.344480,B=0.228516,A=1.000000)" :Option%2019 "(R=0.192708,G=0.176606,B=0.115424,A=1.000000)" :Option%2020 "(R=0.109375,G=0.100236,B=0.065511,A=1.000000)") true))))
      (Variables|/Script/UMG.TextBlock|SetText (Variables|/Game/Widget/W_InfoJournee.W_InfoJournee_C|GetHourOfTheDay _w_info_journee) (Utilities|Text|ToText(Integer) (Variables|Default|GetHour%20of%20the%20day)))
      (Variables|/Script/UMG.TextBlock|SetText (Variables|/Game/Widget/W_InfoJournee.W_InfoJournee_C|GetMinuteOfTheHour _w_info_journee) (Utilities|Text|ToText(Integer) (Variables|Default|GetMinute%20of%20the%20hour)))
      (if (== (Variables|Default|GetHour%20of%20the%20day) 20)
        (Class|UserWidget|PlayAnimationReverse _w_info_journee_2 (Variables|/Game/Widget/W_InfoJournee.W_InfoJournee_C|Getpaupieres _w_info_journee_2) 1.0 false)
        (Utilities|FlowControl|Delay 3.5)
        (Game|OpenLevel(byObjectReference) "/Game/ThirdPerson/Lvl_ThirdPerson.Lvl_ThirdPerson")
        (else
          (bind _outactors (Actor|GetAllActorswithInterface "/Game/Gestion/BPI_Hour.BPI_Hour_C"))
          (for _array_element _outactors
            (Class|BPIHour|NewHour(Message) _array_element (Variables|Default|GetHour%20of%20the%20day) (Variables|Default|GetMinute%20of%20the%20hour))))))))

(event Custom|Stop%20Timeline
  (Utilities|Time|PauseTimerbyHandle (Variables|Default|GetTimeline)))

(event Custom|Reprendre%20timeline
  (Utilities|Time|UnpauseTimerbyHandle (Variables|Default|GetTimeline)))

(event Custom|Start%20Timeline
  (params (W%20info%20journee :type W%20Info%20Journee%20Object%20Reference))
  (Variables|Default|SetW%20info%20journee W%20info%20journee)
  (bind _returnvalue (Utilities|Time|SetTimerbyEvent (delegate Custom|Day%20Tic) 2.0 true false 2.0))
  (Variables|Default|SetTimeline _returnvalue)
  (Variables|Default|SetHour%20of%20the%20day 6)
  (Variables|Default|SetMinute%20of%20the%20hour 0))

(event EventBeginPlay
  (bind _returnvalue (Actor|GetActorOfClass "/Script/Engine.DirectionalLight"))
  (bind _output_get (Variables|Default|SetDirection%20light _returnvalue))
  (Rendering|Components|Light|SetLightColor (Variables|/Script/Engine.Light|GetLightComponent _output_get) "(R=0.458333,G=0.423423,B=0.288845,A=1.000000)" true))

(fn ConstructionScript)